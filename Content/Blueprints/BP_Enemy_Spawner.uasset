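; BP_Enemy_Spawner periodically spawns BP_Pawn_Enemy pawns at randomly chosen spawn points.
; On BeginPlay it starts a looping timer at EnemySpawnRate and stores the handle.
; Each timer tick picks a random actor from TPEnemySpawnPoints and spawns an enemy at its location with zero rotation, skipping if the array is empty.
; THSpawnerToggle pauses or resumes spawning through the stored timer handle.
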(event `self.ReceiveBeginPlay`
  (bind _returnvalue (`KismetSystemLibrary.K2_SetTimerDelegate` (delegate `Enemy_Spawn`) (`self.Enemy_Spawn_Rate`) true))
  (set `self.TH_Enemy_Spawn` _returnvalue))

(event `Enemy_Spawn`
  (bind _tp_enemy_spawn_points (`self.TP_Enemy_Spawn_Points`))
  (if (> (`KismetArrayLibrary.Array_Length` (`self.TP_Enemy_Spawn_Points`)) 0)
    (`|SpawnActorFromClass` "/Game/Blueprints/BP_Pawn_Enemy.BP_Pawn_Enemy_C" (`KismetMathLibrary.MakeTransform` (`self.K2_GetActorLocation` (`|GetArrayItem` _tp_enemy_spawn_points (`KismetMathLibrary.RandomIntegerInRange` 0 (`KismetArrayLibrary.Array_LastIndex` _tp_enemy_spawn_points))))) "Undefined" "MultiplyWithRoot" null null)))

(fn `TH_Spawner_Toggle`
  (params (is_need_spawn :type Boolean))
  (if is_need_spawn
    (`KismetSystemLibrary.K2_UnPauseTimerHandle` (`self.TH_Enemy_Spawn`))
    (else
      (`KismetSystemLibrary.K2_PauseTimerHandle` (`self.TH_Enemy_Spawn`)))))

(fn `UserConstructionScript`)