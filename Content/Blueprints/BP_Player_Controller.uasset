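; Player controller that runs cursor-based XP pickup, the match countdown and the level-up pause.
; On BeginPlay it caches player state and HUD, shows the cursor and starts two looping timers.
; One timer sphere-overlaps XP cubes under the cursor and passes them to player state; the other sends formatted remaining time to the HUD.
; Level-up events pause these timers and every enemy spawner's timer, then call a still-empty upgrade card deck stub.
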(event `self.ReceiveBeginPlay`
  (`|ExecutionSequence`
    (:`then_0`
      ; // !!! Initializations
      (bind _asbp_player_state (cast `/Game/Blueprints/BP_Player_State` (`GameplayStatics.GetPlayerState` 0)))
      (set `self.Player_State` _asbp_player_state)
      (bind _asbp_hud (cast `/Game/Blueprints/BP_HUD` (`self.GetHUD`)))
      (set `self.HUD` _asbp_hud)
      (`WidgetBlueprintLibrary.SetInputMode_GameAndUIEx` self null)
      (set `self.bShowMouseCursor` true))
    (:`then_1`
      ; Exp Collector
      (bind _returnvalue (`KismetSystemLibrary.K2_SetTimerDelegate` (delegate `Event_EXP_Collector`) 0.2 true))
      (bind _output_get (set `self.TH_Exp_Collector` _returnvalue))
      (`KismetArrayLibrary.Array_Add` (`self.TH_Array`) _output_get)
      ; Game Timer
      (bind _returnvalue_2 (`KismetSystemLibrary.K2_SetTimerDelegate` (delegate `Game_Timer`) 1.0 true))
      (bind _output_get_2 (set `self.TH_Game_Timer` _returnvalue_2))
      (`KismetArrayLibrary.Array_Add` (`self.TH_Array`) _output_get_2)
      ; If Level Up
      (add `/Game/Blueprints/BP_Player_State.On_Level_Up` (`self.Player_State`) (delegate `Level_Up_Handler`)))))

(event `Level_Up_Handler`
  ; If Level Up
  (`self.Game_Pause`) ; Game timer and collector for now
  (`self.Spawner_Pause`)
  (`self.Create_Card_Deck_Upgrades`))

(event `Event_EXP_Collector`
  ; Exp Collector
  (bind _exp_count (`self.Exp_Collect_Sphere_Radius` 200.0))
  (`/Game/Blueprints/BP_Player_State.Set_Exp` (`self.Player_State`) _exp_count))

(event `Game_Timer`
  ; Game Timer
  (bind _newparam (`self.Float_To_Text` (`self.Game_Time_Remain`)))
  (`/Game/Blueprints/BP_HUD.Game_Timer_Toggle` (`self.HUD`) _newparam))

(fn `Create_Card_Deck_Upgrades`
  (return))

(fn `Exp_Collect_Sphere_Radius`
  (params (exp_radius_collect :type "Float (single-precision)"))
  (returns (exp_count :type "Array of Actor Object Reference"))
  (locals (collect_radius :type "Float (single-precision)") (amount :type "Float (double-precision)"))
  (set `local.collect_radius` exp_radius_collect)
  (bind _outactors (`KismetSystemLibrary.SphereOverlapActors` (`.Location` (`GameplayStatics.BreakHitResult` (`self.GetHitResultUnderCursorByChannel` "TraceTypeQuery1"))) (`local.collect_radius`) (`|MakeArray` "ObjectTypeQuery1" :!type "EObjectTypeQuery Enum") "/Game/Blueprints/BP_XP_Cube.BP_XP_Cube_C"))
  (return _outactors))

(fn `Float_To_Text`
  (params (game_time_remain_ref :type "Float (double-precision) (by ref)"))
  (returns (NewParam :type Text))
  (bind _result (`/Engine/EditorBlueprintResources/StandardMacros.DecrementFloat` game_time_remain_ref)
    (:`  `
      (return (`|FormatText` "{m}:{s}" (`KismetTextLibrary.Conv_DoubleToText` (`KismetMathLibrary.Conv_IntToDouble` (`KismetMathLibrary.FTrunc` (/ _result 60.0))) "HalfToEven" false true 2) (`KismetTextLibrary.Conv_DoubleToText` (`KismetMathLibrary.Conv_IntToDouble` (`KismetMathLibrary.FTrunc` (mod _result 60.0))) "HalfToEven" false true 2))))))

(fn `Game_Pause`
  (for _array_element (`self.TH_Array`)
    (`KismetSystemLibrary.K2_PauseTimerHandle` _array_element))
  (return))

(fn `Spawner_Pause`
  ; // !!! Need in next frame
  (bind _outactors (`GameplayStatics.GetAllActorsOfClass` "/Game/Blueprints/BP_Enemy_Spawner.BP_Enemy_Spawner_C"))
  (for _array_element _outactors
    (`KismetSystemLibrary.K2_PauseTimerHandle` (`/Game/Blueprints/BP_Enemy_Spawner.TH_Enemy_Spawn` _array_element)))
  (return))

(fn `UserConstructionScript`)