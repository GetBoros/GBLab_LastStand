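; Player pawn that automatically kills enemies, as in an auto-attack survivor-style game.
; A looping timer started on BeginPlay scans all BP_Pawn_Enemy actors for the closest one and draws a debug line to it.
; That target is destroyed instantly, with no projectile, and a BP_XP_Cube spawns at its transform.
; Enemies overlapping Damage_Zone are also destroyed, but drop no XP cube.
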(event `self.ReceiveBeginPlay`
  (`KismetSystemLibrary.K2_SetTimerDelegate` (delegate `Enemy_Find_Destroy`) 2.0 true))

(event `Enemy_Find_Destroy`
  (bind _enemy_closest (`self.Find_Enemy_Closest`))
  (`/Engine/EditorBlueprintResources/StandardMacros.IsValid` _enemy_closest
    (:`Is Valid`
      (`self.Fire_Enemy` _enemy_closest))))

(event `self.Damage_Zone.OnComponentBeginOverlap`
  (params (OverlappedComponent :type "PrimitiveComponent Object Reference") (OtherActor :type "Actor Object Reference") (OtherComp :type "PrimitiveComponent Object Reference") (OtherBodyIndex :type Integer) (bFromSweep :type Boolean) (SweepResult :type "HitResult Structure (by ref)"))
  (bind _asbp_pawn_enemy (cast `/Game/Blueprints/BP_Pawn_Enemy` OtherActor))
  (`self.K2_DestroyActor` _asbp_pawn_enemy))

(fn `Find_Enemy_Closest`
  (returns (Enemy_Closest :type "/Game/Blueprints/BP_Pawn_Enemy Object Reference"))
  (locals (enemy_distance_min :type "Float (double-precision)" :default 999999.0))
  ; Comment
  (bind _outactors (`GameplayStatics.GetAllActorsOfClass` "/Game/Blueprints/BP_Pawn_Enemy.BP_Pawn_Enemy_C"))
  (for _array_element _outactors
    (set `self.Enemy_Distance` (`KismetMathLibrary.Vector_Distance` (`self.K2_GetActorLocation`) (`self.K2_GetActorLocation` _array_element)))
    (if (< (`self.Enemy_Distance`) (`local.enemy_distance_min`))
      (set `local.enemy_distance_min` (`self.Enemy_Distance`))
      (set `self.Enemy_Closest` _array_element)))
  ; Comment
  (bind _enemy_closest (`self.Enemy_Closest`)
    (:`then`
      (`KismetSystemLibrary.DrawDebugLine` (`self.K2_GetActorLocation` self) (`self.K2_GetActorLocation` _enemy_closest) (struct :`R` 0.050492 :`G` 0.062386 :`B` 1.0 :`A` 1.0) 0.5 5.0)
      (return (`self.Enemy_Closest`)))
    (:`else`
      (return null))))

(fn `Fire_Enemy`
  (params (Target :type "Actor Object Reference"))
  (`|SpawnActorFromClass` "/Game/Blueprints/BP_XP_Cube.BP_XP_Cube_C" (`self.GetTransform` Target) "Undefined" "MultiplyWithRoot" null null)
  (`self.K2_DestroyActor` Target)
  (return))

(fn `UserConstructionScript`)