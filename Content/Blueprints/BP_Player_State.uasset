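; BP_Player_State tracks the player's health, experience and level, broadcasting changes through event dispatchers.
; SetExp adds each XP cube's value to current experience, then destroys the cube.
; A while loop resolves multiple level-ups at once, carrying surplus experience over and growing the next threshold geometrically.
; HealthDamageApply subtracts damage, announces the health change and returns whether health is depleted.
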(fn `Health_Damage_Apply`
  (params (damage :type "Float (double-precision)"))
  (returns (is_death :type Boolean))
  (set `self.Health_Current` (- (`self.Health_Current`) damage))
  (`self.On_Health_Change`)
  (return (<= (`self.Health_Current`) 0.0)))

(fn `Set_Exp`
  (params (exp_actors :type "Array of Actor Object Reference"))
  (locals (exp_cube :type "/Game/Blueprints/BP_XP_Cube Object Reference"))
  ; Comment
  (for _array_element exp_actors
    (bind _asbp_xp_cube (cast `/Game/Blueprints/BP_XP_Cube` _array_element))
    (set `local.exp_cube` _asbp_xp_cube)
    (bind _output_get (set `self.Exp_Current` (+ (`/Game/Blueprints/BP_XP_Cube.Exp_Count` (`local.exp_cube`)) (`self.Exp_Current`))))
    (while (>= _output_get (`self.Exp_Level_Next`))
      (set `self.Exp_Current` (- (`self.Exp_Current`) (`self.Exp_Level_Next`)))
      (set `self.Level` (+ (`self.Level`) 1.0))
      (set `self.Exp_Level_Next` (* (`self.Exp_Level_Next`) 1.1))
      (`self.On_Level_Up`))
    (`self.On_Exp_Change`)
    (`self.K2_DestroyActor` (`local.exp_cube`))))

(fn `UserConstructionScript`)